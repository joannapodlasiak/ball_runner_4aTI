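; BP_Ball_01 is a rolling ball pawn that counts a score when its sphere overlaps something.
; Both movement axes feed one torque call on the Sphere, applying the input scaled by StrMulti to X and Y together as an acceleration change.
; Any sphere overlap increments and prints Score; the tagged BP_Crystal_01 search and always-true branch do not filter what counts.
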(event `InputAxis|MoveForwardBack`
  (params (AxisValue :type "Float (single-precision)"))
  (bind _strmulti (`self.StrMulti`))
  (`PrimitiveComponent.AddTorqueInRadians` (`self.Sphere`) (`KismetMathLibrary.MakeVector` (* (stale `InputAxis|MoveLeftRight` AxisValue) _strmulti) (* AxisValue _strmulti)) "None" true :!label _label))

(event `InputAxis|MoveLeftRight`
  (params (AxisValue :type "Float (single-precision)"))
  (goto _label))

(event `self.Sphere.OnComponentBeginOverlap`
  (params (OverlappedComponent :type "PrimitiveComponent Object Reference") (OtherActor :type "Actor Object Reference") (OtherComp :type "PrimitiveComponent Object Reference") (OtherBodyIndex :type Integer) (bFromSweep :type Boolean) (SweepResult :type "HitResult Structure (by ref)"))
  (`GameplayStatics.GetAllActorsOfClassWithTag` "/Game/Blueprints/Actors/BP_Crystal_01.BP_Crystal_01_C" "krysztal")
  (if true
    (bind _result (`/Engine/EditorBlueprintResources/StandardMacros.IncrementFloat` (`self.Score`))
      (:`  `
        (bind _output_get (set `self.Score` _result))
        (`KismetSystemLibrary.PrintString` (`KismetStringLibrary.Conv_DoubleToString` _output_get))))))

(fn `UserConstructionScript`)